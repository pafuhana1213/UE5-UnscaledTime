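; Sample actor that compares the standard Delay with UnscaledDelay by lighting two point lights.
; On BeginPlay it adds two hidden point lights offset to opposite sides along Y, then starts both delays together with the same duration.
; Delay reveals the first light, while UnscaledDelay, set to tick while paused, reveals the second, exposing any timing difference between them.
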(event EventBeginPlay
  (bind _returnvalue (AddComponent|AddPointLightComponent false))
  (Transformation|SetRelativeLocation _returnvalue (Math|Vector|MakeVector 0.0 -1.6e+02 2e+02) false false)
  (Rendering|SetVisibility _returnvalue false false)
  (bind _returnvalue_2 (AddComponent|AddPointLightComponent false))
  (Transformation|SetRelativeLocation _returnvalue_2 (Math|Vector|MakeVector 0.0 1.6e+02 2e+02) false false)
  (Rendering|SetVisibility _returnvalue_2 false false)
  (Utilities|FlowControl|Sequence
    (:then_0
      (Utilities|FlowControl|Delay 3.0)
      (Rendering|SetVisibility _returnvalue true false))
    (:then_1
      (Class|UnscaledTimeBlueprintLibrary|UnscaledDelay 3.0 true)
      (Rendering|SetVisibility _returnvalue_2 true false))))

(event Collision|EventActorBeginOverlap
  (params (OtherActor :type Actor%20Object%20Reference)))

(event EventTick
  (params (DeltaSeconds :type Float%20%28single-precision%29)))

(fn ConstructionScript)