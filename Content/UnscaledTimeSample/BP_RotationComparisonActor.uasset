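; Sample actor that visually compares scaled and unscaled delta time using two spinning cubes.
; BeginPlay creates the normal and unscaled cube mesh components at runtime, offset to either side of the actor.
; Tick yaws both at the same rate, one using Tick's DeltaSeconds and the other GetUnscaledDeltaSeconds, so their rotations diverge when the two deltas differ, as under time dilation.
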(event EventBeginPlay
  (bind _returnvalue (AddComponent|AddStaticMeshComponent false))
  (Components|StaticMesh|SetStaticMesh _returnvalue "/Engine/BasicShapes/Cube.Cube")
  (Transformation|SetRelativeLocation _returnvalue (Math|Vector|MakeVector 0.0 -1.6e+02 1e+02) false false)
  (Variables|Default|SetNormalCube _returnvalue)
  (bind _returnvalue_2 (AddComponent|AddStaticMeshComponent false))
  (Components|StaticMesh|SetStaticMesh _returnvalue_2 "/Engine/BasicShapes/Cube.Cube")
  (Transformation|SetRelativeLocation _returnvalue_2 (Math|Vector|MakeVector 0.0 1.6e+02 1e+02) false false)
  (Variables|Default|SetUnscaledCube _returnvalue_2))

(event Collision|EventActorBeginOverlap
  (params (OtherActor :type Actor%20Object%20Reference)))

(event EventTick
  (params (DeltaSeconds :type Float%20%28single-precision%29))
  (Transformation|AddLocalRotation (Variables|Default|GetNormalCube) (Math|Rotator|MakeRotator 0.0 0.0 (* DeltaSeconds (Math|Float|MakeLiteralFloat 9e+01))) false false)
  (Transformation|AddLocalRotation (Variables|Default|GetUnscaledCube) (Math|Rotator|MakeRotator 0.0 0.0 (* (Class|UnscaledTimeBlueprintLibrary|GetUnscaledDeltaSeconds) (Math|Float|MakeLiteralFloat 9e+01))) false false))

(fn ConstructionScript)