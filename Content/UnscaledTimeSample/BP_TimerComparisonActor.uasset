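; BP_TimerComparisonActor is a sample actor that compares a standard looping timer with an unscaled-time timer.
; On BeginPlay it creates two side-by-side text render components and starts both timers at the same interval, using SetTimerByFunctionName and SetUnscaledTimer.
; Each timer callback increments its own counter and writes it to its text, making any difference between the two tick counts visible in the world.
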(event EventBeginPlay
  (bind _self self)
  (bind _returnvalue (AddComponent|AddTextRenderComponent false))
  (Variables|Default|SetVanillaText _returnvalue)
  (Transformation|SetRelativeLocation _returnvalue (Math|Vector|MakeVector 0.0 -1.6e+02 1.2e+02) false false)
  (Rendering|Components|TextRender|SetWorldSize _returnvalue 64.0)
  (Rendering|Components|TextRender|SetText _returnvalue (Utilities|Text|ToText(String) "V:0"))
  (bind _returnvalue_2 (AddComponent|AddTextRenderComponent false))
  (Variables|Default|SetUnscaledText _returnvalue_2)
  (Transformation|SetRelativeLocation _returnvalue_2 (Math|Vector|MakeVector 0.0 1.6e+02 1.2e+02) false false)
  (Rendering|Components|TextRender|SetWorldSize _returnvalue_2 64.0)
  (Rendering|Components|TextRender|SetText _returnvalue_2 (Utilities|Text|ToText(String) "U:0"))
  (Utilities|Time|SetTimerbyFunctionName _self "OnVanillaTimer" 1.0 true)
  (Class|UnscaledTimeBlueprintLibrary|SetUnscaledTimer _self "OnUnscaledTimer" 1.0 true true))

(event Collision|EventActorBeginOverlap
  (params (OtherActor :type Actor%20Object%20Reference)))

(event EventTick
  (params (DeltaSeconds :type Float%20%28single-precision%29)))

(fn ConstructionScript)

(fn OnVanillaTimer
  (Variables|Default|SetVanillaCount (+ (Variables|Default|GetVanillaCount) (Class|KismetSystemLibrary|MakeLiteralInteger 1)))
  (Rendering|Components|TextRender|SetText (Variables|Default|GetVanillaText) (Utilities|Text|ToText(Integer) (Variables|Default|GetVanillaCount))))

(fn OnUnscaledTimer
  (Variables|Default|SetUnscaledCount (+ (Variables|Default|GetUnscaledCount) (Class|KismetSystemLibrary|MakeLiteralInteger 1)))
  (Rendering|Components|TextRender|SetText (Variables|Default|GetUnscaledText) (Utilities|Text|ToText(Integer) (Variables|Default|GetUnscaledCount))))